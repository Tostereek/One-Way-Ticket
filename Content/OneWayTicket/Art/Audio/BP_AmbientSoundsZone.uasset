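; Ambient audio zone that plays random sounds at varying positions within a sphere, after random delays.
; Sphere overlap, or the player already being inside at BeginPlay, starts the timer; end overlap clears it.
; SetNewSound prepares one reused audio component with random sound, navmesh-reachable location, volume and pitch.
; When a sound finishes, it prepares the next and restarts the timer without rechecking overlap.
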(event `self.ReceiveBeginPlay`
  (`parent.ReceiveBeginPlay`)
  (`self.SetNewSound`)
  (`KismetSystemLibrary.DelayUntilNextTick`)
  (if (`KismetArrayLibrary.Array_IsNotEmpty` (`self.GetOverlappingActors` "/Game/OneWayTicket/Blueprints/Characters/PlayerCharacter/BP_PlayerCharacter.BP_PlayerCharacter_C"))
    (`self.SetTimerForPlayAmbientSound`)))

(event `OnSoundFinished`
  (`self.SetNewSound`)
  (`self.SetTimerForPlayAmbientSound`))

(event `self.SphereZone.OnComponentBeginOverlap`
  (params (OverlappedComponent :type "PrimitiveComponent Object Reference") (OtherActor :type "Actor Object Reference") (OtherComp :type "PrimitiveComponent Object Reference") (OtherBodyIndex :type Integer) (bFromSweep :type Boolean) (SweepResult :type "HitResult Structure (by ref)"))
  (`self.SetTimerForPlayAmbientSound`))

(event `self.SphereZone.OnComponentEndOverlap`
  (params (OverlappedComponent :type "PrimitiveComponent Object Reference") (OtherActor :type "Actor Object Reference") (OtherComp :type "PrimitiveComponent Object Reference") (OtherBodyIndex :type Integer))
  (`KismetSystemLibrary.K2_ClearAndInvalidateTimerHandle` (`self.PlayAmbientSound_TimerHandle`)))

(fn `GetRandomLocationInSphere`
  (returns (RandomLocation :type "Vector Structure"))
  (return (`NavigationSystemV1.K2_GetRandomReachablePointInRadius` (`SceneComponent.K2_GetComponentLocation` (`self.SphereZone`)) (`SphereComponent.SphereRadius` (`self.SphereZone`)) null null)))

(fn `PlayAmbientSound`
  (locals (T :type "Float (double-precision)" :default 0.0))
  (`AudioComponent.Stop` (`self.SpawnedSoundComponent`))
  (`AudioComponent.Play` (`self.SpawnedSoundComponent`) 0.0)
  (return))

(fn `SetNewSound`
  (if (`KismetArrayLibrary.Array_IsNotEmpty` (`self.Sounds`))
    (`AudioComponent.SetSound` (`self.SpawnedSoundComponent`) (`KismetArrayLibrary.Array_Random` (`self.Sounds`)))
    (add `AudioComponent.OnAudioFinished` (`self.SpawnedSoundComponent`) (`|CreateDelegate` :!event `OnSoundFinished`))
    (`SceneComponent.K2_SetWorldLocation` (`self.SpawnedSoundComponent`) (`self.GetRandomLocationInSphere`) false false)
    (`AudioComponent.SetVolumeMultiplier` (`self.SpawnedSoundComponent`) (`KismetMathLibrary.RandomFloatInRange` (`self.MinVolume`) (`self.MaxVolume`)))
    (`AudioComponent.SetPitchMultiplier` (`self.SpawnedSoundComponent`) (`KismetMathLibrary.RandomFloatInRange` (`self.MinPitch`) (`self.MaxPitch`)))
    (return)
    (else
      (return))))

(fn `SetTimerForPlayAmbientSound`
  (bind _returnvalue (`KismetSystemLibrary.K2_SetTimerDelegate` (`|CreateDelegate` :!event `PlayAmbientSound`) (`KismetMathLibrary.RandomFloatInRange` (`self.MinDelay`) (`self.MaxDelay`))))
  (set `self.PlayAmbientSound_TimerHandle` _returnvalue)
  (return))

(fn `UserConstructionScript`)