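; BP_SoundTrigger is a box trigger that has a chance to play a configurable sound when overlapped.
; BeginPlay assigns the sound and attenuation to its AudioComponent and binds the finished event.
; A successful roll plays the sound and locks the trigger, while a failed roll leaves it ready for the next overlap.
; A cooldown timer starts when playback finishes and re-enables the trigger when it expires.
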(event `self.BoxCollision.OnComponentBeginOverlap`
  (params (OverlappedComponent :type "PrimitiveComponent Object Reference") (OtherActor :type "Actor Object Reference") (OtherComp :type "PrimitiveComponent Object Reference") (OtherBodyIndex :type Integer) (bFromSweep :type Boolean) (SweepResult :type "HitResult Structure (by ref)"))
  (if (`self.CanTrigger`)
    (if (<= (`KismetMathLibrary.RandomFloatInRange` 0.0 1.0) (`self.TriggerChance`))
      (`AudioComponent.Play` (`self.AudioComponent`) 0.0)
      (set `self.CanTrigger` false))))

(event `self.ReceiveBeginPlay`
  (`AudioComponent.SetSound` (`self.AudioComponent`) (`self.SoundToPlay`))
  (set `AudioComponent.AttenuationSettings` (`self.Attenuation`) (`self.AudioComponent`))
  (add `AudioComponent.OnAudioFinished` (`self.AudioComponent`) (delegate `OnAudioFinished`)))

(event `OnAudioFinished`
  (`KismetSystemLibrary.K2_SetTimerDelegate` (delegate `OnCooldownEnd`) (`self.Cooldown`)))

(event `OnCooldownEnd`
  (set `self.CanTrigger` true))

(fn `UserConstructionScript`)