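; Blueprint function library of shared helper functions for OneWayTicket.
; It offers a percentage-based random bool roll and typed getters that cast the game instance and game mode to the project's Blueprint classes.
; An on-screen check projects a world position through player 0's controller and tests whether the normalized screen coordinates fall inside the viewport.
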(fn `GetGameInstance`
  (returns (GameInstance :type "/Game/OneWayTicket/Blueprints/Game/BP_GameInstance Object Reference"))
  (bind _asbp_game_instance (cast `/Game/OneWayTicket/Blueprints/Game/BP_GameInstance` (`GameplayStatics.GetGameInstance` null)))
  (return _asbp_game_instance))

(fn `GetGameMode`
  (returns (GameMode :type "/Game/OneWayTicket/Blueprints/Game/BP_GameMode Object Reference"))
  (bind _asbp_game_mode (cast `/Game/OneWayTicket/Blueprints/Game/BP_GameMode` (`GameplayStatics.GetGameMode` null)))
  (return _asbp_game_mode))

(fn `IsLocatedOnScreen`
  (params (InWorldPosition :type "Vector Structure (by ref)"))
  (returns (bIsOnScreen :type Boolean))
  (locals (PC :type "PlayerController Object Reference") (SizeX :type Integer :default 0) (SizeY :type Integer :default 0) (SPX :type "Float (double-precision)" :default 0.0) (SPY :type "Float (double-precision)" :default 0.0))
  (bind _screenposition (`GameplayStatics.ProjectWorldToScreen` (`local.PC`) (`local.InWorldPosition`)))
  (bind _returnvalue (/ (`local.SPY`) (`local.SizeY`)))
  (bind _returnvalue_2 (/ (`local.SPX`) (`local.SizeX`)))
  (bind _output_get (set `local.PC` (`GameplayStatics.GetPlayerController` null)))
  (bind (_sizex _sizey) (`PlayerController.GetViewportSize` _output_get))
  (set `local.SizeX` _sizex)
  (set `local.SizeY` _sizey)
  (set `local.SPX` (`KismetMathLibrary.BreakVector2D` _screenposition))
  (set `local.SPY` (`.Y` (`KismetMathLibrary.BreakVector2D` _screenposition)))
  (return (and (> _returnvalue_2 0.0) (< _returnvalue_2 1.0) (> _returnvalue 0.0) (< _returnvalue 1.0))))

(fn `RandomBoolWithChance`
  (params (InPercentageChance :type "Float (double-precision)" :default 50.0))
  (returns (Outcome :type Boolean))
  (return (>= InPercentageChance (`KismetMathLibrary.RandomFloatInRange` 0.0 100.0))))