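; Player character Blueprint that drives camera shake and tracks an Insanity value.
; Each Tick starts the idle shake while velocity is at or below max walk speed, and the walk shake only above it.
; UpdateInsanity raises Insanity by a small step scaled by the incoming multiplier and prints the total.
; GetInsanity returns the current value.
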(event `self.ReceiveTick`
  (params (DeltaSeconds :type "Float (single-precision)"))
  (`parent.ReceiveTick` DeltaSeconds)
  (`self.ShakeCamera`))

(event `/Game/OneWayTicket/Blueprints/Interfaces/BPI_Player.UpdateInsanity`
  (params (InInsanityMultiplier :type "Float (double-precision)"))
  (bind _output_get (set `self.Insanity` (+ (`self.Insanity`) (* 0.1 InInsanityMultiplier))))
  (`KismetSystemLibrary.PrintString` (`KismetStringLibrary.Conv_DoubleToString` _output_get)))

(fn `GetInsanity`
  (returns (Insanity :type "Float (double-precision)"))
  (return (`self.Insanity`)))

(fn `ShakeCamera`
  (if (<= (`KismetMathLibrary.VSize` (`self.GetVelocity`)) (`CharacterMovementComponent.MaxWalkSpeed` (`self.CharacterMovement`)))
    (`PlayerCameraManager.StartCameraShake` :`self` (`GameplayStatics.GetPlayerCameraManager` 0) :`ShakeClass` "/Game/OneWayTicket/Blueprints/Characters/PlayerCharacter/CameraShake/BP_CameraShakeIdle.BP_CameraShakeIdle_C")
    (else
      (`PlayerCameraManager.StartCameraShake` :`self` (`GameplayStatics.GetPlayerCameraManager` 0) :`ShakeClass` "/Game/OneWayTicket/Blueprints/Characters/PlayerCharacter/CameraShake/BP_CameraShakeWalk.BP_CameraShakeWalk_C"))))

(fn `UserConstructionScript`)