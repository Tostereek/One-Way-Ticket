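; BP_SaveSettings is a settings data container in the One Way Ticket save system, holding the game's audio, video and controls settings.
; Each category lives in its own variable behind a plain setter and getter pair, with no validation, applying or disk access in these functions.
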(fn `GetAudioSettings`
  (returns (AudioSettings :type "/Game/OneWayTicket/Blueprints/Data/SAudioSettings Structure"))
  (return (`self.AudioSettings`)))

(fn `GetControlsSettings`
  (returns (ControlsSettings :type "/Game/OneWayTicket/Blueprints/Data/SControlsSettings Structure"))
  (return (`self.ControlsSettings`)))

(fn `GetVideoSettings`
  (returns (VideoSettings :type "/Game/OneWayTicket/Blueprints/Data/SVideoSettings Structure"))
  (return (`self.VideoSettings`)))

(fn `SetAudioSettings`
  (params (InAudioSettings :type "/Game/OneWayTicket/Blueprints/Data/SAudioSettings Structure"))
  (set `self.AudioSettings` InAudioSettings)
  (return))

(fn `SetControlsSettings`
  (params (InControlsSettings :type "/Game/OneWayTicket/Blueprints/Data/SControlsSettings Structure"))
  (set `self.ControlsSettings` InControlsSettings)
  (return))

(fn `SetVideoSettings`
  (params (InVideoSettings :type "/Game/OneWayTicket/Blueprints/Data/SVideoSettings Structure"))
  (set `self.VideoSettings` InVideoSettings)
  (return))