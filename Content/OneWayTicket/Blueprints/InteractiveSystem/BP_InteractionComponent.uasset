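; Character interaction component that lets the owner use nearby BPI_Interactable actors through press, hold or multi-tap input.
; Capsule overlaps maintain an in-range list, with the most recently added actor as the active interactable.
; A runtime-created screen-space widget component shows WBP_Interact at that actor's location, displaying hold or tap progress.
; IA_Interact branches on the interactable's type, binding dispatchers for holds, then sends the Interact interface message.
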(event `self.ReceiveBeginPlay`
  (`self.CacheOwner`)
  (add `PrimitiveComponent.OnComponentBeginOverlap` (`Character.CapsuleComponent` (`self.Owner`)) (`|CreateDelegate` :!event `HandleCapsuleOverlapBegin`))
  (add `PrimitiveComponent.OnComponentEndOverlap` (`Character.CapsuleComponent` (`self.Owner`)) (`|CreateDelegate` :!event `HandleCapsuleOverlapEnd`))
  (bind _returnvalue (`|AddComponentByClass` :`self` (`self.GetOwner`) :`Class` "/Script/UMG.WidgetComponent" :`bManualAttachment` true))
  (`WidgetComponent.SetWidgetSpace` _returnvalue "Screen")
  (`WidgetComponent.SetDrawSize` _returnvalue (270.0 30.0))
  (set `self.InteractionWidgetComponent` _returnvalue))

(event `HandleCapsuleOverlapBegin`
  (params (OverlappedComponent :type "PrimitiveComponent Object Reference") (OtherActor :type "Actor Object Reference") (OtherComp :type "PrimitiveComponent Object Reference") (OtherBodyIndex :type Integer) (bFromSweep :type Boolean) (SweepResult :type "HitResult Structure (by ref)"))
  (if (`KismetSystemLibrary.DoesImplementInterface` OtherActor "/Game/OneWayTicket/Blueprints/InteractiveSystem/BPI_Interactable.BPI_Interactable_C")
    (`KismetArrayLibrary.Array_AddUnique` (`self.InteractablesInRange`) OtherActor)
    (`self.RenderInteractionWidget`)))

(event `HandleCapsuleOverlapEnd`
  (params (OverlappedComponent :type "PrimitiveComponent Object Reference") (OtherActor :type "Actor Object Reference") (OtherComp :type "PrimitiveComponent Object Reference") (OtherBodyIndex :type Integer))
  (if (`KismetSystemLibrary.DoesImplementInterface` OtherActor "/Game/OneWayTicket/Blueprints/InteractiveSystem/BPI_Interactable.BPI_Interactable_C")
    (if (== OtherActor (`self.GetActiveInteractable`))
      (`self.ResetInteractionState`))
    (`KismetArrayLibrary.Array_RemoveItem` (`self.InteractablesInRange`) OtherActor)
    (`self.RenderInteractionWidget`)))

(event `EnhancedInput|/Game/OneWayTicket/Inputs/InputActions/IA_Interact`
  (params (ActionValue :type Boolean) (ElapsedSeconds :type "Float (double-precision)") (TriggeredSeconds :type "Float (double-precision)") (InputAction :type "InputAction Object Reference" :default "/Game/OneWayTicket/Inputs/InputActions/IA_Interact.IA_Interact"))
  (:`Started`
    (`self.InteractBegin`))
  (:`Ongoing`
    (`self.OnInteractionPressOngoing` ElapsedSeconds))
  (:`Canceled`
    (clear `self.OnInteractionPressOngoing` :!label _label)
    (`self.OnInteractionEnded`))
  (:`Completed`
    (goto _label)))

(event `ResetWidgetProgress`
  (bind _interactionwidget (`self.InteractionWidget`)
    (:`then`
      (`/Game/OneWayTicket/Blueprints/InteractiveSystem/WBP_Interact.SetProgressPercent` _interactionwidget 0.0)
      (remove `self.OnInteractionEnded` (delegate `ResetWidgetProgress`)))
    (:`else`)))

(event `InteractBegin`
  (bind _activeinteractable (`self.GetActiveInteractable`))
  (`/Engine/EditorBlueprintResources/StandardMacros.IsValid` _activeinteractable
    (:`Is Valid`
      (bind _interactiontype (message `/Game/OneWayTicket/Blueprints/InteractiveSystem/BPI_Interactable.GetInteractionType` _activeinteractable))
      (switch `/Game/OneWayTicket/Blueprints/InteractiveSystem/E_InteractionType` _interactiontype
        (:`NewEnumerator0`
          (`self.InteractWithActiveInteractable`))
        (:`NewEnumerator1`
          (add `self.OnInteractionPressOngoing` (delegate `InteractionOngoing`))
          (add `self.OnInteractionEnded` (delegate `ResetWidgetProgress`)))
        (:`NewEnumerator2`
          (`self.InteractionTap`))))))

(event `InteractionOngoing` :!signature `self.OnInteractionPressOngoing`
  (params (ElapsedSeconds :type "Float (double-precision)"))
  (bind _activeinteractable (`self.GetActiveInteractable`))
  (`/Engine/EditorBlueprintResources/StandardMacros.IsValid` _activeinteractable
    (:`Is Valid`
      (bind _duration (message `/Game/OneWayTicket/Blueprints/InteractiveSystem/BPI_Interactable.GetHoldDuration` _activeinteractable))
      (bind _interactionwidget (`self.InteractionWidget`)
        (:`then`
          (`/Game/OneWayTicket/Blueprints/InteractiveSystem/WBP_Interact.SetProgressPercent` _interactionwidget (/ ElapsedSeconds _duration)))
        (:`else`
          _))
      (if (> ElapsedSeconds _duration)
        (`self.InteractWithActiveInteractable`)
        (remove `self.OnInteractionPressOngoing` (delegate `InteractionOngoing`))))))

(event `InteractionTap`
  (`GameplayStatics.PlaySound2D` "/Engine/VREditor/Sounds/UI/Gizmo_Handle_Clicked.Gizmo_Handle_Clicked" 1.0 1.0 0.0 null null)
  (`/Engine/EditorBlueprintResources/StandardMacros.IncrementInt` (`self.CurrentTapCount`)
    (:`  `
      (bind _value (message `/Game/OneWayTicket/Blueprints/InteractiveSystem/BPI_Interactable.GetTapCount` (`self.GetActiveInteractable`)))
      (if (<= _value 0)
        (`self.InteractWithActor` null)
        (else
          (bind _interactionwidget (`self.InteractionWidget`)
            (:`then`
              (`/Game/OneWayTicket/Blueprints/InteractiveSystem/WBP_Interact.SetProgressPercent` _interactionwidget (/ (`self.CurrentTapCount`) _value))
              (if (>= (`self.CurrentTapCount`) _value)
                (`self.InteractWithActiveInteractable`)))
            (:`else`)))))))

(event `InteractWithActiveInteractable`
  (if (`KismetArrayLibrary.Array_IsNotEmpty` (`self.InteractablesInRange`))
    (message `/Game/OneWayTicket/Blueprints/InteractiveSystem/BPI_Interactable.Interact` (`self.GetActiveInteractable`) (`self.GetOwner`))))

(fn `CacheOwner`
  (bind _ascharacter (cast `Character` (`self.GetOwner`)))
  (set `self.Owner` _ascharacter)
  (return))

(fn `GetActiveInteractable`
  (returns (ActiveInteractable :type "Actor Object Reference"))
  (bind _interactablesinrange (`self.InteractablesInRange`))
  (if (`KismetArrayLibrary.Array_IsNotEmpty` (`self.InteractablesInRange`))
    (return (`|GetArrayItem` _interactablesinrange (`KismetArrayLibrary.Array_LastIndex` _interactablesinrange)))))

(fn `InteractWithActor`
  (params (InActor :type "Actor Object Reference"))
  (`/Engine/EditorBlueprintResources/StandardMacros.IsValid` InActor
    (:`Is Valid`
      (message `/Game/OneWayTicket/Blueprints/InteractiveSystem/BPI_Interactable.Interact` (`local.InActor`) (`GameplayStatics.GetPlayerCharacter` 0))
      (return))
    (:`Is Not Valid`
      (return))))

(fn `RenderInteractionWidget`
  (bind _activeinteractable (`self.GetActiveInteractable`))
  (bind _interactionwidgetcomponent (`self.InteractionWidgetComponent`))
  (`/Engine/EditorBlueprintResources/StandardMacros.IsValid` _activeinteractable
    (:`Is Valid`
      (bind _interactiontype (message `/Game/OneWayTicket/Blueprints/InteractiveSystem/BPI_Interactable.GetInteractionType` _activeinteractable))
      (bind _returnvalue (`|CreateWidget` "/Game/OneWayTicket/Blueprints/InteractiveSystem/WBP_Interact.WBP_Interact_C" null _interactiontype))
      (bind _output_get (set `self.InteractionWidget` _returnvalue))
      (`WidgetComponent.SetWidget` _interactionwidgetcomponent _output_get)
      (`SceneComponent.K2_SetWorldLocation` _interactionwidgetcomponent (`Actor.K2_GetActorLocation` (`self.GetActiveInteractable`)) false false))
    (:`Is Not Valid`
      (`WidgetComponent.SetWidget` (`self.InteractionWidgetComponent`) null))))

(fn `ResetInteractionState`
  (remove `self.OnInteractionPressOngoing` (`|CreateDelegate` :!event `InteractionOngoing`))
  (set `self.CurrentTapCount` 0))