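; BP_InteractableBase is a base Blueprint for interactable world objects in the interaction system.
; Its default Interact response destroys the actor.
; Getters expose the interaction type, hold duration and tap count, describing how the interaction is performed.
; A sphere component has a begin-overlap event, but it contains no logic, and the construction script is empty.
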(event `/Game/OneWayTicket/Blueprints/InteractiveSystem/BPI_Interactable.Interact`
  (params (Interactor :type "Actor Object Reference"))
  (`self.K2_DestroyActor` self))

(event `self.Sphere.OnComponentBeginOverlap`
  (params (OverlappedComponent :type "PrimitiveComponent Object Reference") (OtherActor :type "Actor Object Reference") (OtherComp :type "PrimitiveComponent Object Reference") (OtherBodyIndex :type Integer) (bFromSweep :type Boolean) (SweepResult :type "HitResult Structure (by ref)")))

(fn `GetHoldDuration`
  (returns (Duration :type "Float (double-precision)"))
  (return (`self.HoldDuration`)))

(fn `GetInteractionType`
  (returns (InteractionType :type "/Game/OneWayTicket/Blueprints/InteractiveSystem/E_InteractionType Enum"))
  (return (`self.Interaction Type`)))

(fn `GetTapCount`
  (returns (Value :type Integer))
  (return (`self.TapAmount`)))

(fn `UserConstructionScript`)