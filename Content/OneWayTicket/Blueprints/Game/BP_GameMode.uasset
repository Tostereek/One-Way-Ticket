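; Game mode that runs the anomaly and insanity loop, enables recording during play, and starts ambient audio.
; It tracks active anomalies as gameplay tags from EventManager events, adjusting an insanity multiplier as each activates or deactivates.
; StartGameplayLoop spawns the Wraith and starts a looping timer for UpdatePlayerInsanity, which also runs on anomaly changes.
; While anomalies are active, that update messages the player character and selects an ambient track by insanity tier.
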(event `self.ReceiveBeginPlay`
  (`parent.ReceiveBeginPlay`)
  (`VisualLoggerKismetLibrary.EnableRecording` true)
  (add `EventManager.OnActivatedAnomaly` (subsystem `EventManager`) (`|CreateDelegate` :!event `OnActivatedAnomaly`))
  (add `EventManager.OnDeactivatedAnomaly` (subsystem `EventManager`) (`|CreateDelegate` :!event `OnDeactivatedAnomaly`))
  (`self.CacheAmbientMenager`)
  (bind _ambientmenager (`self.AmbientMenager`)
    (:`then`
      (`/Game/OneWayTicket/Blueprints/Actors/BP_AmbientMenager.PlayAmbient` _ambientmenager))
    (:`else`
      (`KismetSystemLibrary.PrintString` "AmbientManager isn't valid!"))))

(event `self.ReceiveEndPlay`
  (params (EndPlayReason :type "EEndPlayReason Enum" :default "Destroyed"))
  (`parent.ReceiveEndPlay` EndPlayReason)
  (`VisualLoggerKismetLibrary.EnableRecording` false))

(event `OnActivatedAnomaly`
  (params (ActivatedEventActor :type "Actor Object Reference"))
  (bind _returnvalue (message `EventObjectInterface.GetEventObjectTagType` ActivatedEventActor))
  (if (not (`BlueprintGameplayTagLibrary.MatchesAnyTags` _returnvalue (`self.ActivatedAnomalies`) true))
    (`BlueprintGameplayTagLibrary.AddGameplayTag` (`self.ActivatedAnomalies`) _returnvalue)
    (`self.IncreaseMultiplierInsanity` 0.1)
    (`/Engine/EditorBlueprintResources/StandardMacros.IncrementInt` (`self.NumActivatedAnomalies`)
      (:`  `
        (`self.UpdatePlayerInsanity`)))))

(event `OnDeactivatedAnomaly`
  (params (ActivatedEventActor :type "Actor Object Reference"))
  (bind _returnvalue (message `EventObjectInterface.GetEventObjectTagType` ActivatedEventActor))
  (if (`BlueprintGameplayTagLibrary.MatchesAnyTags` _returnvalue (`self.ActivatedAnomalies`) true)
    (`BlueprintGameplayTagLibrary.RemoveGameplayTag` (`self.ActivatedAnomalies`) _returnvalue)
    (`self.DecreasedMultiplierInsanity` 0.1)
    (`/Engine/EditorBlueprintResources/StandardMacros.DecrementInt` (`self.NumActivatedAnomalies`)
      (:`  `
        (`self.UpdatePlayerInsanity`)))))

(fn `CacheAmbientMenager`
  (bind _outactors (`GameplayStatics.GetAllActorsOfClass` "/Game/OneWayTicket/Blueprints/Actors/BP_AmbientMenager.BP_AmbientMenager_C"))
  (set `self.AmbientMenager` (`|GetArrayItem` _outactors)))

(fn `DecreasedMultiplierInsanity`
  (params (InSub :type "Float (double-precision)" :default 1.0))
  (set `self.InsanityMultipier` (- (`self.InsanityMultipier`) (`local.InSub`)))
  (return))

(fn `IncreaseMultiplierInsanity`
  (params (InAdd :type "Float (double-precision)" :default 1.0))
  (set `self.InsanityMultipier` (+ (`self.InsanityMultipier`) (`local.InAdd`)))
  (return))

(fn `StartGameplayLoop`
  (`EventManager.SpawnWraith` (subsystem `EventManager`))
  (bind _returnvalue (`KismetSystemLibrary.K2_SetTimer` null "UpdatePlayerInsanity" 1.0 true))
  (set `self.UpdatePlayerInsanity_TimerHandle` _returnvalue))

(fn `UpdatePlayerInsanity`
  (if (> (`self.NumActivatedAnomalies`) 0)
    (message `/Game/OneWayTicket/Blueprints/Interfaces/BPI_Player.UpdateInsanity` (`GameplayStatics.GetPlayerCharacter` 0) (`self.InsanityMultipier`))
    (bind _insanity (message `/Game/OneWayTicket/Blueprints/Interfaces/BPI_Player.GetInsanity` (`GameplayStatics.GetPlayerCharacter` 0)))
    (if (< _insanity 25.0)
      (`/Game/OneWayTicket/Blueprints/Actors/BP_AmbientMenager.ChangeCurrentAmbient` (`self.AmbientMenager`) "/Game/OneWayTicket/Art/Audio/Music/A_Ambient_01.A_Ambient_01")
      (elif (< _insanity 50.0)
        (`/Game/OneWayTicket/Blueprints/Actors/BP_AmbientMenager.ChangeCurrentAmbient` (`self.AmbientMenager`) "/Game/OneWayTicket/Art/Audio/Music/A_Ambient_02.A_Ambient_02")
        (elif (< _insanity 75.0)
          (`/Game/OneWayTicket/Blueprints/Actors/BP_AmbientMenager.ChangeCurrentAmbient` (`self.AmbientMenager`) "/Game/OneWayTicket/Art/Audio/Music/A_Ambient_03.A_Ambient_03")
          (elif (< _insanity 100.0)
            (`/Game/OneWayTicket/Blueprints/Actors/BP_AmbientMenager.ChangeCurrentAmbient` (`self.AmbientMenager`) "/Game/OneWayTicket/Art/Audio/Music/A_Ambient_04.A_Ambient_04")))))))

(fn `UserConstructionScript`)