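; Player controller that handles first-person-style look and movement input and toggles the pause menu.
; On begin play it adds the IMC_Player Enhanced Input context and reads mouse sensitivity from the game instance.
; Look and move actions drive the player character along its forward and right vectors.
; The pause action lazily creates WBP_Pause, then shows or hides it while switching game pause, cursor and input mode.
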(event `self.ReceiveBeginPlay`
  (`parent.ReceiveBeginPlay`)
  (`EnhancedInputSubsystemInterface.AddMappingContext` (subsystem `EnhancedInputLocalPlayerSubsystem`) "/Game/OneWayTicket/Inputs/IMC_Player.IMC_Player" 0 (struct))
  (set `self.MouseSensitivity` (`/Game/OneWayTicket/Blueprints/Game/BP_GameInstance.MouseSensitivity` (`/Game/OneWayTicket/Blueprints/FunctionLibraries/BPFL_HelperFunctions.GetGameInstance`))))

(event `EnhancedInput|/Game/OneWayTicket/Inputs/InputActions/IA_Look`
  (params (ActionValue :type "Vector2D Structure") (ElapsedSeconds :type "Float (double-precision)") (TriggeredSeconds :type "Float (double-precision)") (InputAction :type "InputAction Object Reference" :default "/Game/OneWayTicket/Inputs/InputActions/IA_Look.IA_Look"))
  (:`Triggered`
    (`Pawn.AddControllerYawInput` (`GameplayStatics.GetPlayerCharacter` 0) (* ActionValue_X (`self.MouseSensitivity`)))
    (`Pawn.AddControllerPitchInput` (`GameplayStatics.GetPlayerCharacter` 0) (* ActionValue_Y (`self.MouseSensitivity`)))))

(event `EnhancedInput|/Game/OneWayTicket/Inputs/InputActions/IA_Move`
  (params (ActionValue :type "Vector2D Structure") (ElapsedSeconds :type "Float (double-precision)") (TriggeredSeconds :type "Float (double-precision)") (InputAction :type "InputAction Object Reference" :default "/Game/OneWayTicket/Inputs/InputActions/IA_Move.IA_Move"))
  (:`Triggered`
    (`Pawn.AddMovementInput` (`GameplayStatics.GetPlayerCharacter` 0) (`self.GetActorRightVector` (`GameplayStatics.GetPlayerCharacter` 0)) ActionValue_X false)
    (`Pawn.AddMovementInput` (`GameplayStatics.GetPlayerCharacter` 0) (`self.GetActorForwardVector` (`GameplayStatics.GetPlayerCharacter` 0)) ActionValue_Y false)))

(event `EnhancedInput|/Game/OneWayTicket/Inputs/InputActions/IA_Pause`
  (params (ActionValue :type Boolean) (ElapsedSeconds :type "Float (double-precision)") (TriggeredSeconds :type "Float (double-precision)") (InputAction :type "InputAction Object Reference" :default "/Game/OneWayTicket/Inputs/InputActions/IA_Pause.IA_Pause"))
  (:`Started`
    (`self.PauseWidget`
      (:`then`
        (if (`GameplayStatics.IsGamePaused`)
          (`self.HidePauseMenu`)
          (else
            (`self.DisplayPauseMenu`))))
      (:`else`
        (bind _returnvalue (`|CreateWidget` "/Game/OneWayTicket/Blueprints/Widgets/Interface/WBP_Pause.WBP_Pause_C"))
        (set `self.PauseWidget` _returnvalue)
        (`self.DisplayPauseMenu`)))))

(fn `DisplayPauseMenu`
  (`UserWidget.AddToViewport` (`self.PauseWidget`) 0)
  (`GameplayStatics.SetGamePaused` true)
  (set `PlayerController.bShowMouseCursor` true (`GameplayStatics.GetPlayerController` 0))
  (`WidgetBlueprintLibrary.SetInputMode_GameAndUIEx` (`GameplayStatics.GetPlayerController` 0) (`self.PauseWidget`))
  (return))

(fn `HidePauseMenu`
  (`Widget.RemoveFromParent` (`self.PauseWidget`))
  (`GameplayStatics.SetGamePaused` false)
  (set `PlayerController.bShowMouseCursor` false (`GameplayStatics.GetPlayerController` 0))
  (`WidgetBlueprintLibrary.SetInputMode_GameOnly` (`GameplayStatics.GetPlayerController` 0))
  (return))

(fn `UserConstructionScript`)