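; BP_Speaker is a speaker actor that plays a report sound at its location when game event objects update.
; On BeginPlay it binds to the EventManager's event-object update callback.
; For each update it looks up the object by ID and, if active, queries its type through an interface.
; That type keys a Reports map to pick the sound to spawn, which is stored as ReportSound.
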(event `self.ReceiveBeginPlay`
  (add `EventManager.OnUpdateEventObject` (subsystem `EventManager`) (`|CreateDelegate` :!event `CustomEvent`)))

(event `CustomEvent`
  (params (EventObjectID :type "Guid Structure"))
  (bind _returnvalue (`EventManager.FindEventObjectViewById` (subsystem `EventManager`) EventObjectID))
  (bind ((`Interface` _interface)) (break `EventObjectView` _returnvalue))
  (bind _returnvalue_2 (`EventObjectInterface.IsEventObjectActive` _interface))
  (if _returnvalue_2
    (bind _returnvalue_3 (`EventObjectInterface.GetEventObjectType` _interface))
    (bind _returnvalue_4 (`GameplayStatics.SpawnSoundAtLocation` (`BlueprintMapLibrary.Map_Find` (`/Game/OneWayTicket/Blueprints/Data/PDA_SpeakerReports.Reports` (`self.Reports`)) _returnvalue_3) (`self.K2_GetActorLocation`) (struct) 1.0 1.0 0.0 null null))
    (set `self.ReportSound` _returnvalue_4)))

(fn `UserConstructionScript`)