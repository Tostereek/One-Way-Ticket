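; Anomaly Blueprint that makes an assigned set of lamps flicker while it is active.
; Activation starts a looping timer at the flicker frequency, and ToggleLights gives each lamp a random chance to flip its event-object state.
; Deactivation clears the timer and switches every lamp off.
; The construction script draws temporary debug lines above the assigned lamps to mark them.
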(event `self.OnActivated`
  (`parent.OnActivated`)
  (`self.SetTimerForToggleLights`))

(event `self.OnDeactivated`
  (`parent.OnDeactivated`)
  (`KismetSystemLibrary.K2_ClearAndInvalidateTimerHandle` (`self.ToggleLights_TimerHandle`))
  (`self.DeactivateAllLamps`))

(fn `DeactivateAllLamps`
  (for _array_element (`self.Lamps`)
    (`self.DeactivateEventObject` _array_element))
  (return))

(fn `SetTimerForToggleLights`
  (bind _returnvalue (`KismetSystemLibrary.K2_SetTimerDelegate` (`|CreateDelegate` :!event `ToggleLights`) (`self.FlickingFrequency`) true))
  (set `self.ToggleLights_TimerHandle` _returnvalue)
  (return))

(fn `ToggleLights`
  (locals (LampFromArray :type "EventObject Object Reference"))
  (for _array_element (`self.Lamps`)
    (set `local.LampFromArray` _array_element)
    (if (`KismetMathLibrary.RandomBool`)
      (bind _returnvalue (`EventObjectInterface.IsEventObjectActive` (`local.LampFromArray`)))
      (if _returnvalue
        (`self.DeactivateEventObject` (`local.LampFromArray`))
        (else
          (`self.ActivateEventObject` (`local.LampFromArray`))))))
  (return))

(fn `UserConstructionScript`
  (for _array_element (`self.Lamps`)
    (bind _returnvalue (`self.K2_GetActorLocation` _array_element))
    (`KismetSystemLibrary.DrawDebugLine` (+ _returnvalue (0.0 0.0 1000.0)) _returnvalue (struct :`R` 1.0 :`G` 0.002732 :`B` 0.799103 :`A` 1.0) 5.0 20.0)))