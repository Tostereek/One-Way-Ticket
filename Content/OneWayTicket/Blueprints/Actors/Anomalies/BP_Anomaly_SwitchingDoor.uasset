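; Anomaly actor that randomly changes the state of an assigned set of doors while it is active.
; Activation starts a looping timer running SwitchDoors, which uses a chance roll to either open each door or toggle its mesh; deactivation clears the timer.
; When the array holds at most one door, a fallback closes it if DoorSwitched is false.
; The construction script draws colored debug lines above each door and its dependent doors.
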(event `self.OnActivated`
  (`parent.OnActivated`)
  (bind _returnvalue (`KismetSystemLibrary.K2_SetTimer` null "SwitchDoors" 1.0 true)))

(event `self.OnDeactivated`
  (`parent.OnDeactivated`)
  (`KismetSystemLibrary.K2_ClearAndInvalidateTimerHandle` (stale `self.OnActivated` _returnvalue)))

(fn `SwitchDoors`
  (locals (bDoorSwitched :type Boolean) (DoorFromArray :type "/Game/OneWayTicket/Blueprints/Actors/Malfunction/BP_Malfunction_Door Object Reference"))
  (bind _doorfromarray (`local.DoorFromArray`))
  (for _array_element (`self.Doors`)
    (set `local.DoorFromArray` _array_element)
    (bind _outcome (`/Game/OneWayTicket/Blueprints/FunctionLibraries/BPFL_HelperFunctions.RandomBoolWithChance` (`self.ChanceToChangeDoor`)))
    (if _outcome
      (`/Game/OneWayTicket/Blueprints/Actors/Malfunction/BP_Malfunction_Door.OpenDoor` _doorfromarray)
      (else
        (`/Game/OneWayTicket/Blueprints/Actors/Malfunction/BP_Malfunction_Door.ToggleMesh` _doorfromarray))))
  (if (and (<= (`KismetArrayLibrary.Array_Length` (`self.Doors`)) 1) (not (`local.bDoorSwitched`)))
    (`/Game/OneWayTicket/Blueprints/Actors/Malfunction/BP_Malfunction_Door.CloseDoor` (`KismetArrayLibrary.Array_Random` (`self.Doors`)))))

(fn `UserConstructionScript`
  (`parent.UserConstructionScript`)
  (for _array_element (`self.Doors`)
    (bind _returnvalue (`self.K2_GetActorLocation` _array_element))
    (`KismetSystemLibrary.DrawDebugLine` (+ _returnvalue (0.0 0.0 1000.0)) _returnvalue (struct :`R` 1.0 :`G` 0.002732 :`B` 0.799103 :`A` 1.0) 5.0 20.0)
    (for _array_element_2 (`/Game/OneWayTicket/Blueprints/Actors/Malfunction/BP_Malfunction_Door.DependetDoors` _array_element)
      (bind _returnvalue_2 (`self.K2_GetActorLocation` _array_element_2))
      (`KismetSystemLibrary.DrawDebugLine` (+ _returnvalue_2 (0.0 0.0 1000.0)) _returnvalue_2 (struct :`R` 1.0 :`G` 0.873948 :`A` 1.0) 5.0 20.0))))