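; BP_Anomaly_AlterRoom is an anomaly that alters a room by swapping level meshes for its own when activated.
; On BeginPlay it caches all of its StaticMeshComponents as the anomaly meshes.
; On activation it hides the actors in MeshesFromLevel0 and disables their mesh collision, then shows the cached meshes with query and physics collision.
; The swap has no reversal in this Blueprint, and both events call their parent implementations first.
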(event `self.ReceiveBeginPlay`
  (`parent.ReceiveBeginPlay`)
  (for _array_element (`self.K2_GetComponentsByClass` "/Script/Engine.StaticMeshComponent")
    (`KismetArrayLibrary.Array_Add` (`self.AnomalyMeshes`) _array_element)))

(event `self.OnActivated`
  (`parent.OnActivated`)
  (for _array_element (`self.MeshesFromLevel_0`)
    (`SceneComponent.SetHiddenInGame` (`Actor.RootComponent` _array_element) true false)
    (`PrimitiveComponent.SetCollisionEnabled` (`self.GetComponentByClass` _array_element "/Script/Engine.StaticMeshComponent") "NoCollision"))
  (for _array_element_2 (`self.AnomalyMeshes`)
    (`SceneComponent.SetHiddenInGame` _array_element_2 false false)
    (`PrimitiveComponent.SetCollisionEnabled` _array_element_2 "QueryAndPhysics")))

(fn `UserConstructionScript`)