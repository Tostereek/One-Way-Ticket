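; Shelf malfunction actor in OneWayTicket, currently a skeleton on top of its parent class.
; BeginPlay runs the parent logic, then gathers the static mesh components and checks each for the "Drawer" tag, with no action on a match.
; The construction script is empty, and GetEventObjectId returns without a visible value.
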(event `self.ReceiveBeginPlay`
  (`parent.ReceiveBeginPlay`)
  (set `self.MeshComponents` (`self.K2_GetComponentsByClass` "/Script/Engine.StaticMeshComponent"))
  (if (not (`KismetArrayLibrary.Array_IsEmpty` (`self.MeshComponents`)))
    (for _array_element (`self.MeshComponents`)
      (if (`ActorComponent.ComponentHasTag` _array_element "Drawer")
        _))))

(fn `GetEventObjectId`
  (returns (ReturnValue :type "Guid Structure"))
  (return))

(fn `UserConstructionScript`)