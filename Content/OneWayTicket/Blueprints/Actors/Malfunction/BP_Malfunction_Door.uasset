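; Malfunction door actor that slides two wings open and closed as the player enters or leaves its box trigger, and locks while the malfunction is active.
; A timeline drives both wings in mirrored directions and updates the open state on finish, with checks on open, locked and wall states gating movement.
; Opening, closing and mesh toggling propagate to dependent doors, and toggling swaps between a door and a locked wall.
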(event `self.ReceiveBeginPlay`
  (`parent.ReceiveBeginPlay`)
  (`TimelineComponent.SetTimelineFinishedFunc` (`self.DoorWings_Interpolation`) (`|CreateDelegate` :!event `OnTimelineFinished`)))

(event `self.OnActivated`
  (`parent.OnActivated`)
  (set `self.bIsLocked` true))

(event `self.OnDeactivated`
  (`parent.OnDeactivated`)
  (set `self.bIsLocked` false))

(event `OpenDoor`
  ; Timeline
  (if (`self.CanOpenDoor`)
    (`self.OnOpen`)
    (bind (_direction _interpolation) (`Timeline|DoorWings_Interpolation` :!label _label)
      (:`Update`
        (bind _returnvalue (`KismetMathLibrary.VLerp` (0.0 0.0 0.0) (0.0 100.0 0.0) _interpolation))
        (`SceneComponent.K2_SetRelativeLocation` (`self.LeftWindMesh`) _returnvalue false false)
        (`SceneComponent.K2_SetRelativeLocation` (`self.RightWindMesh`) (* _returnvalue -1.0) false false)))))

(event `CloseDoor`
  ; Timeline
  (if (`self.CanCloseDoor`)
    (`self.OnClose`)
    (goto _label :!via `ReverseFromEnd`)))

(event `OnTimelineFinished`
  ; Timeline
  (set `self.bIsOpen` (>= (`TimelineComponent.GetPlaybackPosition` (`self.DoorWings_Interpolation`)) (`TimelineComponent.GetTimelineLength` (`self.DoorWings_Interpolation`)))))

(event `OnOpen`
  (`GameplayStatics.PlaySoundAtLocation` (`self.OpenDoorSound`) (`self.K2_GetActorLocation`) (struct) 1.0 1.0 0.0 null null null null)
  (for _array_element (`self.DependetDoors`)
    (`self.OpenDoor` _array_element))
  (`self.OnOpenDoor`))

(event `OnClose`
  (`GameplayStatics.PlaySoundAtLocation` (`self.CloseDoorSound`) (`self.K2_GetActorLocation`) (struct) 1.0 1.0 0.0 null null null null)
  (for _array_element (`self.DependetDoors`)
    (`self.CloseDoor` _array_element))
  (`self.OnCloseDoor`))

(event `self.BoxCollider.OnComponentBeginOverlap`
  (params (OverlappedComponent :type "PrimitiveComponent Object Reference") (OtherActor :type "Actor Object Reference") (OtherComp :type "PrimitiveComponent Object Reference") (OtherBodyIndex :type Integer) (bFromSweep :type Boolean) (SweepResult :type "HitResult Structure (by ref)"))
  (set `self.bIsCollidingWithPlayer` true)
  (if (not (`self.bIsOpen`))
    (`self.OpenDoor`)))

(event `self.BoxCollider.OnComponentEndOverlap`
  (params (OverlappedComponent :type "PrimitiveComponent Object Reference") (OtherActor :type "Actor Object Reference") (OtherComp :type "PrimitiveComponent Object Reference") (OtherBodyIndex :type Integer))
  (set `self.bIsCollidingWithPlayer` false)
  (if (`self.bIsOpen`)
    (`self.CloseDoor`)))

(fn `CanCloseDoor`
  (returns (CanOpen :type Boolean))
  (return (and (`self.bIsOpen`) (not (`self.bIsLocked`)) (not (`self.bIsWall`)))))

(fn `CanOpenDoor`
  (returns (CanOpen :type Boolean))
  (return (`KismetMathLibrary.BooleanNAND` (`self.bIsOpen`) (`self.bIsLocked`) (`self.bIsWall`))))

(fn `ChangeToDoor`
  (`self.SetEventActorMesh` "/Game/OneWayTicket/Art/Enviroment/Ship/SM_Door.SM_Door")
  (set `self.bIsWall` false)
  (set `self.bIsLocked` false)
  (return))

(fn `ChangeToWall`
  (`self.SetEventActorMesh` "/Game/OneWayTicket/Art/Enviroment/Ship/SM_DoorAsWall.SM_DoorAsWall")
  (set `self.bIsWall` true)
  (set `self.bIsLocked` true)
  (return))

(fn `ToggleMesh`
  (for _array_element (`self.DependetDoors`)
    (`self.ToggleMesh` _array_element))
  (if (`self.bIsWall`)
    (`self.ChangeToDoor`)
    (else
      (`self.ChangeToWall`))))

(fn `UserConstructionScript`)