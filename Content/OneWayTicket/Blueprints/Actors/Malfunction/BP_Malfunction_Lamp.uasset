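; BP_Malfunction_Lamp is a malfunction actor for a lamp that goes dark while the malfunction is active.
; It extends a parent malfunction class, calling the parent's activation and deactivation events before its own logic.
; Activation hides the main and additional rect lights through TurnOffLights, and deactivation shows them again through TurnOnLights.
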(event `self.OnActivated`
  (`parent.OnActivated`)
  (`self.TurnOffLights`))

(event `self.OnDeactivated`
  (`parent.OnDeactivated`)
  (`self.TurnOnLights`))

(fn `TurnOffLights`
  (`SceneComponent.SetVisibility` (`self.RectLightAdditional`) false false)
  (`SceneComponent.SetVisibility` (`self.RectLightMain`) false false)
  (return))

(fn `TurnOnLights`
  (`SceneComponent.SetVisibility` (`self.RectLightAdditional`) true false)
  (`SceneComponent.SetVisibility` (`self.RectLightMain`) true false)
  (return))

(fn `UserConstructionScript`)