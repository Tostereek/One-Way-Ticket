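; BP_RotatingObject is a placeable actor that spins a configurable static mesh around its local axes.
; The construction script applies the chosen ObjectStaticMesh to ObjectMesh.
; On BeginPlay, the ObjectRotation timeline starts, and each update adds a local rotation equal to its Rotation output scaled by separate X, Y and Z speeds.
; The rotation step is per update with no delta-time scaling, so spin rate depends on frame rate.
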(event `self.ReceiveBeginPlay`
  (bind (_direction _rotation) (`Timeline|ObjectRotation`)
    (:`Update`
      (`SceneComponent.K2_AddLocalRotation` (`self.ObjectMesh`) (`KismetMathLibrary.MakeRotator` (* _rotation (`self.RotationSpeedX`)) (* _rotation (`self.RotationSpeedY`)) (* _rotation (`self.RotationSpeedZ`))) false false))))

(fn `UserConstructionScript`
  (`StaticMeshComponent.SetStaticMesh` (`self.ObjectMesh`) (`self.ObjectStaticMesh`)))