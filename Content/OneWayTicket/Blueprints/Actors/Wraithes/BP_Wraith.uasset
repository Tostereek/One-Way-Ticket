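; Wraith enemy, drawn as a flipbook sprite, that triggers random anomalies in the level while it exists.
; On BeginPlay it gathers tagged anomalies from the EventManager, then activates inactive ones on a random-interval timer, subject to an active-count limit.
; While on screen, the sprite yaws toward the camera, and player overlap with its sphere runs a looping timer to build Tension.
; Full Tension destroys the wraith, and EndPlay deactivates its active anomalies.
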(event `self.ReceiveBeginPlay`
  (`parent.ReceiveBeginPlay`)
  (bind _output_get (set `self.Anomalies` (`EventManager.FindEventObjectsByTags` (subsystem `EventManager`) (`BlueprintGameplayTagLibrary.MakeLiteralGameplayTagContainer` (`self.AnomalyTypes`)))))
  (if (not (`KismetArrayLibrary.Array_IsEmpty` _output_get))
    (set `self.InactiveAnomalies` (`self.Anomalies`))
    (`self.SetTimerForActivateAnomaly`)
    (else
      (`KismetSystemLibrary.PrintString` "There aren't anomalies!"))))

(event `ActivateAnomaly`
  (if (`self.CheckIfCanActivateAnomaly`)
    (bind _activatedanomaly (`self.ActivateRandomAnomaly`))
    (bind _output_get (set `self.ActiveAnomaly` _activatedanomaly))
    (`/Engine/EditorBlueprintResources/StandardMacros.IsValid` _output_get
      (:`Is Valid`
        (add `EventObject.OnDeactivateEventObject` (`self.ActiveAnomaly`) (`|CreateDelegate` :!event `RemoveActiveAnomalyFromArray`))
        (`EventObject.ActivateEventObject` (`self.ActiveAnomaly`))
        (`self.SetTimerForActivateAnomaly`))
      (:`Is Not Valid`
        (`KismetSystemLibrary.PrintString` "Anomaly isn't valid!")))))

(event `self.ReceiveEndPlay`
  (params (EndPlayReason :type "EEndPlayReason Enum" :default "Destroyed"))
  (`parent.ReceiveEndPlay` EndPlayReason)
  (`self.BanishWraith`))

(event `self.ReceiveTick`
  (params (DeltaSeconds :type "Float (single-precision)"))
  (`parent.ReceiveTick` DeltaSeconds)
  (if (`/Game/OneWayTicket/Blueprints/FunctionLibraries/BPFL_HelperFunctions.IsLocatedOnScreen` (+ (`self.K2_GetActorLocation`) (0.0 0.0 130.0)))
    (`self.FaceToPlayer`)
    (if (`self.bCollideWithPlayer`)
      (if (not (`KismetSystemLibrary.K2_IsTimerActiveHandle` (`self.Timer`)))
        (bind _returnvalue (`KismetSystemLibrary.K2_SetTimerDelegate` (`|CreateDelegate` :!event `IncreaseTension`) 0.1 true))
        (set `self.Timer` _returnvalue))
      (else
        (`KismetSystemLibrary.K2_ClearAndInvalidateTimerHandle` (`self.Timer`))))
    (else
      (`KismetSystemLibrary.K2_ClearAndInvalidateTimerHandle` (`self.Timer`)))))

(event `self.SphereCollider.OnComponentBeginOverlap`
  (params (OverlappedComponent :type "PrimitiveComponent Object Reference") (OtherActor :type "Actor Object Reference") (OtherComp :type "PrimitiveComponent Object Reference") (OtherBodyIndex :type Integer) (bFromSweep :type Boolean) (SweepResult :type "HitResult Structure (by ref)"))
  (set `self.bCollideWithPlayer` true))

(event `self.SphereCollider.OnComponentEndOverlap`
  (params (OverlappedComponent :type "PrimitiveComponent Object Reference") (OtherActor :type "Actor Object Reference") (OtherComp :type "PrimitiveComponent Object Reference") (OtherBodyIndex :type Integer))
  (set `self.bCollideWithPlayer` false)
  (`KismetSystemLibrary.K2_ClearAndInvalidateTimerHandle` (`self.Timer`)))

(event `IncreaseTension`
  (bind _output_get (set `self.Tension` (`KismetMathLibrary.FClamp` (+ (`self.Tension`) 5.0) 0.0 100.0)))
  (if (>= _output_get 100.0)
    (`self.K2_DestroyActor`)))

(fn `ActivateRandomAnomaly`
  (returns (ActivatedAnomaly :type "EventObject Object Reference"))
  (locals (InActiveAnomaly :type "EventObject Object Reference"))
  (bind _output_get (set `local.InActiveAnomaly` (`KismetArrayLibrary.Array_Random` (`self.InactiveAnomalies`))))
  (bind _returnvalue (message `EventObjectInterface.IsEventObjectActive` _output_get))
  (if (not _returnvalue)
    (`KismetArrayLibrary.Array_Add` (`self.ActiveAnomalies`) (`local.InActiveAnomaly`))
    (`KismetArrayLibrary.Array_RemoveItem` (`self.InactiveAnomalies`) (`local.InActiveAnomaly`))
    (`VisualLoggerKismetLibrary.LogText` null (`KismetStringLibrary.Concat_StrStr` "Activated anomaly: " (`KismetSystemLibrary.GetDisplayName` (`local.InActiveAnomaly`))) "LogEventManager")
    (return (`local.InActiveAnomaly`))
    (else
      (`KismetSystemLibrary.PrintString` "Anomaly has not been activated!"))))

(fn `BanishWraith`
  (`KismetSystemLibrary.K2_ClearAndInvalidateTimerHandle` (`self.ActivateAnomaly_TimerHandle`))
  (for _array_element (`self.ActiveAnomalies`)
    (`EventObject.DeactivateEventObject` _array_element))
  (`KismetArrayLibrary.Array_Clear` (`self.ActiveAnomalies`))
  (return))

(fn `CheckIfCanActivateAnomaly`
  (returns (ReturnValue :type Boolean))
  (return (and (<= (`KismetArrayLibrary.Array_Length` (`self.ActiveAnomalies`)) (`self.LimitActiveAnomalies`)) (`KismetArrayLibrary.Array_IsNotEmpty` (`self.InactiveAnomalies`)))))

(fn `FaceToPlayer`
  (`SceneComponent.K2_SetRelativeRotation` (`self.WraithFlipbook`) (`KismetMathLibrary.MakeRotator` 0.0 0.0 (+ (.yaw (`KismetMathLibrary.FindLookAtRotation` (`PlayerCameraManager.GetCameraLocation` (`GameplayStatics.GetPlayerCameraManager` 0)) (`self.K2_GetActorLocation`))) 90.0)) false false)
  (return))

(fn `RemoveActiveAnomalyFromArray`
  (params (InAnomaly :type "EventObject Object Reference"))
  (`KismetArrayLibrary.Array_Add` (`self.InactiveAnomalies`) (`local.InAnomaly`))
  (remove `EventObject.OnDeactivateEventObject` (`local.InAnomaly`) (`|CreateDelegate` :!event `RemoveActiveAnomalyFromArray`))
  (return))

(fn `SetRandomSeedForTimer`
  (returns (ReturnValue :type "Float (single-precision)"))
  (return (`KismetMathLibrary.RandomFloatInRangeFromStream` (`self.Stream`) (`self.MinTimeToActivateAnomaly`) (`self.MaxTimeToActivateAnomaly`))))

(fn `SetTimerForActivateAnomaly`
  (`KismetMathLibrary.SeedRandomStream` (`self.Stream`))
  (bind _returnvalue (`KismetSystemLibrary.K2_SetTimerDelegate` (`|CreateDelegate` :!event `ActivateAnomaly`) (`self.SetRandomSeedForTimer`)))
  (set `self.ActivateAnomaly_TimerHandle` _returnvalue)
  (return))

(fn `UserConstructionScript`)