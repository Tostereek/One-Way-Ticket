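; BP_Computer is an in-world computer actor with a screen widget for showing device status.
; On BeginPlay it gives its WBP_DevicesStatus widget a new controller and binds to EventManager object updates.
; Each update looks up the device's row by ID and sets its active-state indicator.
; ShowDevicesOnScreen's logic for building rows from Malfunction-tagged objects is disconnected, so nothing here fills the Devices map.
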(event `self.ReceiveBeginPlay`
  (`parent.ReceiveBeginPlay`)
  (`self.InitializeScreenWidget`)
  (`self.ShowDevicesOnScreen`)
  (add `EventManager.OnUpdateEventObject` (subsystem `EventManager`) (delegate `CustomEvent`)))

(event `CustomEvent`
  (params (EventObjectID :type "Guid Structure"))
  (`self.UpdateStatus` EventObjectID))

(fn `InitializeScreenWidget`
  (bind _returnvalue (`|GenericCreateObject` "/Game/OneWayTicket/Blueprints/Widgets/BP_WidgetController.BP_WidgetController_C"))
  (set `self.WidgetController` _returnvalue)
  (bind _aswbp_devices_status (cast `/Game/OneWayTicket/Blueprints/Widgets/WBP_DevicesStatus` (`WidgetComponent.GetWidget` (`self.Widget`))))
  (bind _output_get (set `self.ScreenWidget` _aswbp_devices_status))
  (`/Game/OneWayTicket/Blueprints/Widgets/WBP_DevicesStatus.SetWidgetController` _output_get (`self.WidgetController`))
  (return))

(fn `ShowDevicesOnScreen`
  (locals (InDeviceView :type "EventObjectView Structure") (InDeviceRow :type "/Game/OneWayTicket/Blueprints/Widgets/WBP_DeviceStatus Object Reference")))

(fn `UpdateStatus`
  (params (InDeviceID :type "Guid Structure (by ref)"))
  (locals (InRow :type "/Game/OneWayTicket/Blueprints/Widgets/WBP_DeviceStatus Object Reference"))
  (bind (_value _returnvalue) (`BlueprintMapLibrary.Map_Find` (`self.Devices`) InDeviceID))
  (if _returnvalue
    (bind _output_get (set `local.InRow` _value))
    (`/Engine/EditorBlueprintResources/StandardMacros.IsValid` _output_get
      (:`Is Valid`
        (bind _returnvalue_2 (`EventManager.FindEventObjectViewById` (subsystem `EventManager`) (`local.InDeviceID`)))
        (bind _returnvalue_3 (`EventObjectInterface.IsEventObjectActive` (`.Interface` (break `EventObjectView` _returnvalue_2))))
        (`/Game/OneWayTicket/Blueprints/Widgets/WBP_DeviceStatus.SetStatusIndicator` (`local.InRow`) _returnvalue_3))
      (:`Is Not Valid`
        (`KismetSystemLibrary.PrintString` "DeviceRow isn't valid!")))))

(fn `UserConstructionScript`)